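; Conveyor-style filter station that sets a colour filter (red, green or blue) on held trays and passes them on.
; At BeginPlay, a line trace finds the adjacent BP_Container destination.
; On item change, a scanner timeline moves the arm and applies the colour, then a looping timeline waits until the destination frees, reserves it, and lerps the item across for deposit.
; Withdraw cancels transfers and releases reservations; ChangeColour cycles the laser material.
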(event `self.ReceiveBeginPlay`
  (`parent.ReceiveBeginPlay`)
  (`self.Get Neighbour`))

(event `self.Item Changed`
  (params (`Change Type` :type "/Game/Core/EItemChange Enum" :default "NewEnumerator0"))
  (bind _destination (`self.Destination`))
  (bind _destination_2 (`self.Destination`))
  (bind _destination_3 (`self.Destination`))
  ;[1 1 1] Has Item and Valid Destination
  (if (and (`self.Has Destination`) (`self.HasItem`))
    (bind (_direction _z) (`Timeline|Move Scanner` :!via `PlayFromStart`)
      (:`Update`
        (`SceneComponent.K2_SetRelativeLocation` (`self.Arm`) (`KismetMathLibrary.MakeVector` 0.0 0.0 _z) false false))
      (:`Finished`
        ;[1 1 1] Destination Occupied
        (if (or (`/Game/Blueprints/BP_Container.HasItem` _destination_2) (`/Game/Blueprints/BP_Container.Reserved` _destination_2))
          ;[1 1 1] Check Again Loop
          (`Timeline|Check Again` :!via `PlayFromStart`
            (:`Check`
              (if (not (or (`/Game/Blueprints/BP_Container.HasItem` _destination) (`/Game/Blueprints/BP_Container.Reserved` _destination)))
                (`|ExecutionSequence`
                  (:`then_0`
                    (`TimelineComponent.Stop` (`self.Check Again`)))
                  (:`then_1`
                    (set `/Game/Blueprints/BP_Container.Reserved` true (`self.Destination`) :!label _label)
                    (set `self.isReservingOther` true)
                    ;[1 1 1] Move Item
                    (bind (_direction_2 _postion_alpha) (`Timeline|Move Along` :!via `PlayFromStart`)
                      (:`Update`
                        (`self.K2_SetActorLocation` (`self.Item Held`) (`KismetMathLibrary.VLerp` (`SceneComponent.K2_GetComponentLocation` (`self.Scene`)) (`SceneComponent.K2_GetComponentLocation` (`/Game/Blueprints/BP_Container.Scene` (`self.Destination`))) _postion_alpha) false false))
                      (:`Finished`
                        (bind _success (`/Game/BPI/BPI_Interact.Deposit` _destination_3 (`self.Item Held`)))
                        (if _success
                          (set `/Game/Blueprints/BP_Container.Reserved` false _destination_3)
                          (set `self.isReservingOther` false)
                          (set `self.HasItem` false)
                          (set `self.Item Held` null)))))))))
          (else
            (goto _label))))
      (:`Trigger`
        (`/Game/Blueprints/Parts/BP_Part.Set Tray Filter` (`self.Item Held`) true (`self.Colour`))))))

(fn `Change Colour`
  (switch `/Game/Core/EColour` (`self.Colour`)
    (:`NewEnumerator1`
      (set `self.Colour` "NewEnumerator2"))
    (:`NewEnumerator2`
      (set `self.Colour` "NewEnumerator4"))
    (:`NewEnumerator4`
      (set `self.Colour` "NewEnumerator1")))
  (`PrimitiveComponent.SetMaterial` (`self.StaticMesh1`) 0 (select `/Game/Core/EColour` (`self.Colour`) :`NewEnumerator1` "/Game/Materials/Filter/M_Laser_Red.M_Laser_Red" :`NewEnumerator2` "/Game/Materials/Filter/M_Laser_Green.M_Laser_Green" :`NewEnumerator4` "/Game/Materials/Filter/M_Laser_Blue.M_Laser_Blue" :!type "MaterialInstance Object Reference")))

(fn `Get Neighbour`
  (bind _staticmeshcomponent (`self.StaticMeshComponent`))
  (bind _returnvalue (`SceneComponent.K2_GetComponentLocation` _staticmeshcomponent))
  (bind _outhit (`KismetSystemLibrary.LineTraceSingle` (+ _returnvalue (0.0 0.0 10.0)) (+ (- _returnvalue (* (`KismetMathLibrary.GetForwardVector` (`SceneComponent.K2_GetComponentRotation` _staticmeshcomponent)) 100.0)) (0.0 0.0 10.0)) "TraceTypeQuery1"))
  (bind _asbp_container (cast `/Game/Blueprints/BP_Container` (`.HitActor` (`GameplayStatics.BreakHitResult` _outhit)))
    (:`then`
      (set `self.Has Destination` true)
      (set `self.Destination` _asbp_container))
    (:`CastFailed`
      (set `self.Has Destination` false)
      (set `self.Destination` null))))

(fn `UserConstructionScript`
  (`parent.UserConstructionScript`)
  (`PrimitiveComponent.SetMaterial` (`self.StaticMesh1`) 0 (select `/Game/Core/EColour` (`self.Colour`) :`NewEnumerator1` "/Game/Materials/Filter/M_Laser_Red.M_Laser_Red" :`NewEnumerator2` "/Game/Materials/Filter/M_Laser_Green.M_Laser_Green" :`NewEnumerator4` "/Game/Materials/Filter/M_Laser_Blue.M_Laser_Blue" :!type "MaterialInstance Object Reference")))

(fn `Withdraw`
  (returns (Item :type "/Game/Blueprints/Parts/BP_Part Object Reference") (Success :type Boolean))
  (bind _printdebugs (`self.PrintDebugs`))
  (if (`self.HasItem`)
    (`KismetSystemLibrary.PrintString` "Withdraw Success" _printdebugs _printdebugs)
    (set `self.HasItem` false)
    (`TimelineComponent.Stop` (`self.Check Again`))
    (`TimelineComponent.Stop` (`self.Move Along`))
    (`self.Item Changed` "NewEnumerator1")
    (if (`self.isReservingOther`)
      (set `/Game/Blueprints/BP_Container.Reserved` false (`self.Destination`)))
    (return (`self.Item Held`) true)
    (else
      (`KismetSystemLibrary.PrintString` "Withdraw Fail" _printdebugs _printdebugs)
      (return null false))))