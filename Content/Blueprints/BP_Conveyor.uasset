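; Conveyor Blueprint that passes a held item on to a neighbouring BP_Container.
; On BeginPlay, a short line trace against the mesh's forward vector finds and caches that destination.
; When its item changes, it polls a busy destination through a timeline event, then reserves it once free.
; A second timeline lerps the item across, then deposits it and, on success, clears the reservation and its own slot.
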(event `self.ReceiveBeginPlay`
  (`parent.ReceiveBeginPlay`)
  (`self.Get Neighbour`))

(event `self.Item Changed`
  (bind _destination (`self.Destination`))
  (bind _destination_2 (`self.Destination`))
  (bind _destination_3 (`self.Destination`))
  (if (`self.Has Destination`)
    (if (`self.HasItem`)
      (if (or (`/Game/Blueprints/BP_Container.HasItem` _destination_2) (`/Game/Blueprints/BP_Container.Reserved` _destination_2))
        (`Timeline|Check Again` :!via `PlayFromStart` :!label _label
          (:`Check`
            (`KismetSystemLibrary.PrintString` (`KismetStringLibrary.Concat_StrStr` (`KismetSystemLibrary.GetObjectName` self) " is checking"))
            (if (or (`/Game/Blueprints/BP_Container.HasItem` _destination) (`/Game/Blueprints/BP_Container.Reserved` _destination))
              (`KismetSystemLibrary.PrintString` "Destination Occupied")
              (else
                (`|ExecutionSequence`
                  (:`then_0`
                    (goto _label :!via `Stop`))
                  (:`then_1`
                    (set `/Game/Blueprints/BP_Container.Reserved` true (`self.Destination`) :!label _label_2)
                    (`KismetSystemLibrary.PrintString` "Moving Item")
                    (bind (_direction _postion_alpha) (`Timeline|Move Along` :!via `PlayFromStart`)
                      (:`Update`
                        (`self.K2_SetActorLocation` (`self.Item Held`) (`KismetMathLibrary.VLerp` (`SceneComponent.K2_GetComponentLocation` (`self.Scene`)) (`SceneComponent.K2_GetComponentLocation` (`/Game/Blueprints/BP_Container.Scene` (`self.Destination`))) _postion_alpha) false false))
                      (:`Finished`
                        (bind _success (`self.Deposit` _destination_3 (`self.Item Held`)))
                        (if _success
                          (set `/Game/Blueprints/BP_Container.Reserved` false _destination_3)
                          (set `self.HasItem` false)
                          (set `self.Item Held` null))))))))))
        (else
          (goto _label_2))))
    (else
      (`KismetSystemLibrary.PrintString` "No Destination"))))

(fn `Get Neighbour`
  (bind _staticmeshcomponent (`self.StaticMeshComponent`))
  (bind _returnvalue (`SceneComponent.K2_GetComponentLocation` _staticmeshcomponent))
  (bind _outhit (`KismetSystemLibrary.LineTraceSingle` (+ _returnvalue (0.0 0.0 10.0)) (+ (- _returnvalue (* (`KismetMathLibrary.GetForwardVector` (`SceneComponent.K2_GetComponentRotation` _staticmeshcomponent)) 100.0)) (0.0 0.0 10.0)) "TraceTypeQuery1"))
  (bind _asbp_container (cast `/Game/Blueprints/BP_Container` (`.HitActor` (`GameplayStatics.BreakHitResult` _outhit)))
    (:`then`
      (set `self.Has Destination` true)
      (set `self.Destination` _asbp_container))
    (:`CastFailed`
      (set `self.Has Destination` false))))

(fn `UserConstructionScript`
  (`parent.UserConstructionScript`))