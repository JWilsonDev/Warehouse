(event `self.Activate`
  (bind _source (`self.Source`))
  ;[1 1 1] Should Loader Be Active
  (`self.Get Neighbour`)
  (if (`self.Has Source`)
    ;[1 1 1] Look For Item
    (if (`/Game/Blueprints/BP_Container.HasItem` _source) :!label _label
      (if (not (`/Game/Blueprints/BP_Container.Reserved` _source))
        (set `/Game/Blueprints/BP_Container.Reserved` true _source)
        (`TimelineComponent.Stop` (`self.Wait For Item`))
        ;[1 1 1 1 36] Grabber
        (bind (_direction _move) (`Timeline|Move Arm` :!via `PlayFromStart`)
          (:`Update`
            ;;[1 1 1] Move Arm
            (`SceneComponent.K2_SetRelativeLocation` (`self.Arm`) (`KismetMathLibrary.VLerp` (0.0 0.0 0.0) (100.0 0.0 0.0) _move) false false))
          (:`Pickup`
            ;;[1 1 1] Pickup Item
            (bind (_item _success) (`self.Withdraw` (`self.Source`)))
            (bind _output_get (set `self.Item Held` _item))
            (set `self.HasItem` true)
            (if _success
              (`self.K2_AttachToComponent` _output_get (`self.GrabPoint`) "None" "SnapToTarget" "SnapToTarget" "SnapToTarget" true)
              (set `/Game/Blueprints/BP_Container.Reserved` false (`self.Source`))))
          (:`Drop Off`
            ;;[1 1 1] Drop Item On Self
            (`self.K2_AttachToComponent` (`self.Item Held`) (`self.Scene`) "None" "SnapToTarget" "SnapToTarget" "SnapToTarget" true)
            (`self.Move Conveyor`))))
      (else
        (`Timeline|Wait For Item`
          (:`Look Again`
            (goto _label)))))))

(event `Move Conveyor`
  (bind _destination (`self.Destination`))
  (bind _destination_2 (`self.Destination`))
  ;[1 1 1 1 36] Conveyor
  ;;[1 1 1] Has Destination And Item
  (if (and (`self.Has Destination`) (`self.HasItem`))
    ;;[1 1 1] Destination Occupied
    (if (or (`/Game/Blueprints/BP_Container.HasItem` _destination_2) (`/Game/Blueprints/BP_Container.Reserved` _destination_2))
      ;;[1 1 1] Check Again Loop
      (`Timeline|Check Again` :!via `PlayFromStart`
        (:`Check`
          (if (not (or (`/Game/Blueprints/BP_Container.HasItem` _destination) (`/Game/Blueprints/BP_Container.Reserved` _destination)))
            (`|ExecutionSequence`
              (:`then_0`
                (`TimelineComponent.Stop` (`self.Check Again`)))
              (:`then_1`
                (set `/Game/Blueprints/BP_Container.Reserved` true (`self.Destination`) :!label _label_2)
                (set `self.isReservingOther` true)
                ;;[1 1 1] Move Item
                (bind (_direction _postion_alpha) (`Timeline|Move Along` :!via `PlayFromStart`)
                  (:`Update`
                    (`self.K2_SetActorLocation` (`self.Item Held`) (`KismetMathLibrary.VLerp` (`SceneComponent.K2_GetComponentLocation` (`self.Scene`)) (`SceneComponent.K2_GetComponentLocation` (`/Game/Blueprints/BP_Container.Scene` (`self.Destination`))) _postion_alpha) false false))
                  (:`Finished`
                    (bind _success (`self.Deposit` (`self.Destination`) (`self.Item Held`)))
                    (if _success
                      (`self.Withdraw`)))))))))
      (else
        (goto _label_2)))))

(event `self.Item Changed`
  (params (`Change Type` :type "/Game/Core/EItemChange Enum" :default "NewEnumerator0"))
  (bind _move_arm (`self.Move Arm`))
  (bind _move_arm_2 (`self.Move Arm`))
  ;[1 1 1] Item Changed Externally
  (switch `/Game/Core/EItemChange` `Change Type`
    (:`NewEnumerator0`
      (`self.Move Conveyor`))
    (:`NewEnumerator1`
      (bind _output_get (set `self.Arm Position` (.x (.location (`SceneComponent.GetRelativeTransform` (`self.Arm`))))))
      (if (== _output_get 0.0)
        (if (`self.Has Source`)
          (if (`/Game/Blueprints/BP_Container.HasItem` (`self.Source`))
            (`TimelineComponent.PlayFromStart` (`self.Move Arm`))
            (else
              (`TimelineComponent.Play` (`self.Wait For Item`)))))
        (elif (== (`self.Arm Position`) 100.0)
          (`TimelineComponent.SetNewTime` _move_arm_2 2.0)
          (`TimelineComponent.Play` _move_arm_2)
          (elif (`self.Has Source`)
            (if (`/Game/Blueprints/BP_Container.HasItem` (`self.Source`))
              (`TimelineComponent.SetPlayRate` (`self.Return Arm To Pickup`) (/ 100.0 (`self.Arm Position`)))
              (bind (_direction _alpha) (`Timeline|Return Arm To Pickup` :!via `PlayFromStart`)
                (:`Update`
                  (`SceneComponent.K2_SetRelativeLocation` (`self.Arm`) (`KismetMathLibrary.VLerp` (`KismetMathLibrary.MakeVector` (`self.Arm Position`)) (100.0 0.0 0.0) _alpha) false false))
                (:`Finished`
                  (`TimelineComponent.SetNewTime` _move_arm 2.0)
                  (`TimelineComponent.Play` _move_arm)))
              (else
                (`TimelineComponent.SetPlayRate` (`self.Return Arm To Start`) (/ 100.0 (`self.Arm Position`)))
                (bind (_direction_2 _alpha_2) (`Timeline|Return Arm To Start` :!via `PlayFromStart`)
                  (:`Update`
                    (`SceneComponent.K2_SetRelativeLocation` (`self.Arm`) (`KismetMathLibrary.VLerp` (`KismetMathLibrary.MakeVector` (`self.Arm Position`)) (0.0 0.0 0.0) _alpha_2) false false))
                  (:`Finished`
                    (`TimelineComponent.Play` (`self.Wait For Item`))))))))))))

(fn `Deactivate`
  (`TimelineComponent.Stop` (`self.Move Arm`))
  (`TimelineComponent.Stop` (`self.Check Again`))
  (`TimelineComponent.Stop` (`self.Move Along`)))

(fn `Get Neighbour`
  (bind _staticmeshcomponent (`self.StaticMeshComponent`))
  (bind _staticmeshcomponent_2 (`self.StaticMeshComponent`))
  (bind _returnvalue (`SceneComponent.K2_GetComponentLocation` _staticmeshcomponent))
  (bind _returnvalue_2 (`SceneComponent.K2_GetComponentLocation` _staticmeshcomponent_2))
  (bind _outhit (`KismetSystemLibrary.LineTraceSingle` :`Start` (+ _returnvalue_2 (0.0 0.0 10.0)) :`End` (+ (- _returnvalue_2 (* (`KismetMathLibrary.GetForwardVector` (`SceneComponent.K2_GetComponentRotation` _staticmeshcomponent_2)) 100.0)) (0.0 0.0 10.0)) :`TraceChannel` "TraceTypeQuery1" :`DrawDebugType` "Persistent"))
  (bind _asbp_container (cast `/Game/Blueprints/BP_Container` (`.HitActor` (`GameplayStatics.BreakHitResult` _outhit)))
    (:`then`
      (set `self.Has Destination` true)
      (set `self.Destination` _asbp_container))
    (:`CastFailed`
      (set `self.Has Destination` false)
      (set `self.Destination` null)))
  (bind _outhit_2 (`KismetSystemLibrary.LineTraceSingle` :`Start` (+ _returnvalue (0.0 0.0 10.0)) :`End` (+ (+ _returnvalue (* (`KismetMathLibrary.GetForwardVector` (`SceneComponent.K2_GetComponentRotation` _staticmeshcomponent)) 100.0)) (0.0 0.0 10.0)) :`TraceChannel` "TraceTypeQuery1" :`DrawDebugType` "Persistent" :`TraceColor` (struct :`R` 0.150637 :`B` 1.0 :`A` 1.0)))
  (bind _asbp_container_2 (cast `/Game/Blueprints/BP_Container` (`.HitActor` (`GameplayStatics.BreakHitResult` _outhit_2)))
    (:`then`
      (set `self.Has Source` true)
      (set `self.Source` _asbp_container_2))
    (:`CastFailed`
      (set `self.Has Source` false)
      (set `self.Source` null))))

(fn `Rotate`
  (`parent.Rotate`)
  (`SceneComponent.K2_AddWorldRotation` (`self.StaticMesh`) (struct :`Yaw` -90.0) false false))

(fn `UserConstructionScript`
  (`parent.UserConstructionScript`)
  (`SceneComponent.K2_SetWorldRotation` (`self.StaticMesh`) (struct :`Yaw` -90.0 :`Roll` 50.0) false false))

(fn `Withdraw`
  (returns (Item :type "/Game/Blueprints/Parts/BP_Part Object Reference") (Success :type Boolean))
  (bind _printdebugs (`self.PrintDebugs`))
  (if (`self.HasItem`)
    (`KismetSystemLibrary.PrintString` "Withdraw Success" _printdebugs _printdebugs)
    (set `self.HasItem` false)
    (`TimelineComponent.Stop` (`self.Check Again`))
    (`TimelineComponent.Stop` (`self.Move Along`))
    (`TimelineComponent.Stop` (`self.Move Arm`))
    (if (`self.isReservingOther`)
      (set `/Game/Blueprints/BP_Container.Reserved` false (`self.Destination`)))
    (set `self.isReservingOther` false)
    (`self.Item Changed` "NewEnumerator1")
    (return (`self.Item Held`) true)
    (else
      (`KismetSystemLibrary.PrintString` "Withdraw Fail" _printdebugs _printdebugs)
      (return null false))))