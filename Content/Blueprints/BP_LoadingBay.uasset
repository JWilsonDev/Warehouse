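; BP_LoadingBay is a delivery point that generates a random furniture order and accepts items that fulfil it.
; On BeginPlay it fills Order with a random number of random rows from DT_AssembledFurniture.
; Deposit matches type, colour and material, but returns false at the first mismatch, so only the first entry can match.
; A match removes that entry and flags OrderCompleted once Order empties, while Withdraw always fails.
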(event `self.ReceiveBeginPlay`
  (`parent.ReceiveBeginPlay`)
  (set `self.FurnitureData` "/Game/Data_Tables/DT_AssembledFurniture.DT_AssembledFurniture")
  (bind _output_get (set `self.NumberOfItems` (`KismetMathLibrary.RandomIntegerInRange` (`self.MinNumOfItems`) (`self.MaxNumOfItems`))))
  (for _ (range 1 (+ _output_get 1))
    (`self.AddRequiredFurniture`)))

(event `AddRequiredFurniture`
  (bind _furnituredata (`self.FurnitureData`))
  (bind _outrownames (`DataTableFunctionLibrary.GetDataTableRowNames` _furnituredata))
  (bind _returnvalue (`|GetDataTableRow` _furnituredata (`KismetArrayLibrary.Array_Random` _outrownames))
    (:`then`
      (`KismetArrayLibrary.Array_Add` (`self.Order`) _returnvalue))))

(fn `Deposit`
  (params (Item :type "/Game/Blueprints/Parts/BP_Part Object Reference"))
  (returns (Success :type Boolean))
  (locals (CurrentOrderIndex :type Integer))
  (bind _order (`self.Order`))
  (bind (_furnituretype _colour _material) (break `/Game/Core/FFurniture` (`/Game/Blueprints/Parts/BP_Part.FurnitureStructure` Item)))
  (for (_array_element _array_index) (`self.Order`)
    (set `local.CurrentOrderIndex` _array_index)
    (bind (_furnituretype_2 _colour_2 _material_2) (break `/Game/Core/FFurniture` _array_element))
    (if (and (`|EnumEquality` _furnituretype_2 _furnituretype) (`|EnumEquality` _colour_2 _colour) (`|EnumEquality` _material_2 _material))
      (`|ExecutionSequence`
        (:`then_0`
          (break))
        (:`then_1`
          (`KismetArrayLibrary.Array_Remove` _order (`local.CurrentOrderIndex`))
          (if (== (`KismetArrayLibrary.Array_Length` _order) 0)
            (set `self.OrderCompleted` true))
          (return true)))
      (else
        (return false)))))

(fn `UserConstructionScript`
  (`parent.UserConstructionScript`))

(fn `Withdraw`
  (returns (Item :type "/Game/Blueprints/Parts/BP_Part Object Reference") (Success :type Boolean))
  (return null false))