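; BP_Spray is a factory-line station where a robot arm sprays a held item to change its colour, then passes it along.
; On item change, a timeline animates four arm sections and triggers Niagara spray and recolour events.
; It then reserves the container found by a BeginPlay backward line trace, polling while that is occupied, and lerps the item across to deposit it.
; Withdraw cancels the transfer and releases its reservation.
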(event `self.ReceiveBeginPlay`
  (`parent.ReceiveBeginPlay`)
  (`self.Get Neighbour`)
  (`KismetSystemLibrary.Delay` 2.0))

(event `self.Item Changed`
  (params (`Change Type` :type "/Game/Core/EItemChange Enum" :default "NewEnumerator0"))
  (bind _destination (`self.Destination`))
  (bind _destination_2 (`self.Destination`))
  (bind _destination_3 (`self.Destination`))
  (bind (_direction _section_0 _section_1 _section_2 _section_3) (`Timeline|Spray` :!via `PlayFromStart`)
    (:`Update`
      (`SceneComponent.K2_SetRelativeRotation` (`self.RobotArm_Section_0`) (`KismetMathLibrary.MakeRotator` 0.0 0.0 _section_0) false false)
      (`SceneComponent.K2_SetRelativeRotation` (`self.RobotArm_Section_1`) (`KismetMathLibrary.MakeRotator` _section_1) false false)
      (`SceneComponent.K2_SetRelativeRotation` (`self.RobotArm_Section_2`) (`KismetMathLibrary.MakeRotator` _section_2) false false)
      (`SceneComponent.K2_SetRelativeRotation` (`self.RobotArm_Section_3`) (`KismetMathLibrary.MakeRotator` _section_3) false false))
    (:`Finished`
      ;[1 1 1] Has Item and Valid Destination
      (if (and (`self.Has Destination`) (`self.HasItem`))
        ;[1 1 1] Destination Occupied
        (if (or (`/Game/Blueprints/BP_Container.HasItem` _destination_3) (`/Game/Blueprints/BP_Container.Reserved` _destination_3))
          ;[1 1 1] Check Again Loop
          (`Timeline|Check Again` :!via `PlayFromStart`
            (:`Check`
              (if (not (or (`/Game/Blueprints/BP_Container.HasItem` _destination_2) (`/Game/Blueprints/BP_Container.Reserved` _destination_2)))
                (`|ExecutionSequence`
                  (:`then_0`
                    (`TimelineComponent.Stop` (`self.Check Again`)))
                  (:`then_1`
                    ;[1 1 1] Move Item
                    (set `/Game/Blueprints/BP_Container.Reserved` true (`self.Destination`) :!label _label)
                    (set `self.isReservingOther` true)
                    (bind (_direction_2 _postion_alpha) (`Timeline|Move Along` :!via `PlayFromStart`)
                      (:`Update`
                        (`self.K2_SetActorLocation` (`self.Item Held`) (`KismetMathLibrary.VLerp` (`SceneComponent.K2_GetComponentLocation` (`self.Scene`)) (`SceneComponent.K2_GetComponentLocation` (`/Game/Blueprints/BP_Container.Scene` (`self.Destination`))) _postion_alpha) false false))
                      (:`Finished`
                        (bind _success (`/Game/BPI/BPI_Interact.Deposit` _destination (`self.Item Held`)))
                        (if _success
                          (set `/Game/Blueprints/BP_Container.Reserved` false _destination)
                          (set `self.isReservingOther` false)
                          (set `self.HasItem` false)
                          (set `self.Item Held` null)))))))))
          (else
            (goto _label)))))
    (:`Start Spray`
      (`ActorComponent.Activate` (`self.Niagara`) false))
    (:`Stop Spray`
      (`ActorComponent.Deactivate` (`self.Niagara`)))
    (:`Change Colour`
      (`/Game/Blueprints/Parts/BP_Part.Update Part Colour` (`self.Item Held`) (`self.Colour`)))))

(fn `Get Neighbour`
  (bind _staticmeshcomponent (`self.StaticMeshComponent`))
  (bind _returnvalue (`SceneComponent.K2_GetComponentLocation` _staticmeshcomponent))
  (bind _outhit (`KismetSystemLibrary.LineTraceSingle` (+ _returnvalue (0.0 0.0 10.0)) (+ (- _returnvalue (* (`KismetMathLibrary.GetForwardVector` (`SceneComponent.K2_GetComponentRotation` _staticmeshcomponent)) 100.0)) (0.0 0.0 10.0)) "TraceTypeQuery1"))
  (bind _asbp_container (cast `/Game/Blueprints/BP_Container` (`.HitActor` (`GameplayStatics.BreakHitResult` _outhit)))
    (:`then`
      (set `self.Has Destination` true)
      (set `self.Destination` _asbp_container))
    (:`CastFailed`
      (set `self.Has Destination` false)
      (set `self.Destination` null))))

(fn `UserConstructionScript`
  (`parent.UserConstructionScript`))

(fn `Withdraw`
  (returns (Item :type "/Game/Blueprints/Parts/BP_Part Object Reference") (Success :type Boolean))
  (bind _printdebugs (`self.PrintDebugs`))
  (if (`self.HasItem`)
    (`KismetSystemLibrary.PrintString` "Withdraw Success" _printdebugs _printdebugs)
    (set `self.HasItem` false)
    (`TimelineComponent.Stop` (`self.Check Again`))
    (`TimelineComponent.Stop` (`self.Move Along`))
    (`self.Item Changed` "NewEnumerator1")
    (if (`self.isReservingOther`)
      (set `/Game/Blueprints/BP_Container.Reserved` false (`self.Destination`)))
    (return (`self.Item Held`) true)
    (else
      (`KismetSystemLibrary.PrintString` "Withdraw Fail" _printdebugs _printdebugs)
      (return null false))))