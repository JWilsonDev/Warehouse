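; Conveyor sorter that routes a held item to a neighbouring BP_Container on its left, right or front by tray colour.
; Line traces find neighbours at BeginPlay; Sort matches colour, falls back to uncoloured sides, and rotates the chosen entry for round-robin.
; Timelines poll busy destinations, then reserve them and lerp the item across before depositing.
; Side colours cycle through ChangeColour and show as mesh materials; Withdraw cancels transfers.
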(event `self.ReceiveBeginPlay`
  (`parent.ReceiveBeginPlay`)
  (`self.Get Neighbour`))

(event `self.Item Changed`
  (params (`Change Type` :type "/Game/Core/EItemChange Enum" :default "NewEnumerator0"))
  (bind _right (`self.Right`))
  (bind _right_2 (`self.Right`))
  (bind _right_3 (`self.Right`))
  (bind _forward (`self.Forward`))
  (bind _forward_2 (`self.Forward`))
  (bind _forward_3 (`self.Forward`))
  (bind _left (`self.Left`))
  (bind _left_2 (`self.Left`))
  (bind _left_3 (`self.Left`))
  (if (`self.HasItem`)
    (bind _out_side (`self.Sort` (`/Game/Blueprints/Parts/BP_Part.Tray Colour` (`self.Item Held`))))
    (switch `/Game/Core/ESide` _out_side
      (:`NewEnumerator3`
        ;[1 1 1] Destination Occupied
        (if (or (`/Game/Blueprints/BP_Container.HasItem` _left_2) (`/Game/Blueprints/BP_Container.Reserved` _left_2))
          ;[1 1 1] Check Again Loop
          (`Timeline|Check Left` :!via `PlayFromStart`
            (:`Check`
              (if (not (or (`/Game/Blueprints/BP_Container.HasItem` _left_3) (`/Game/Blueprints/BP_Container.Reserved` _left_3)))
                (`|ExecutionSequence`
                  (:`then_0`
                    (`TimelineComponent.Stop` (`self.Check Left`)))
                  (:`then_1`
                    ;[1 1 1] Move Item
                    (set `/Game/Blueprints/BP_Container.Reserved` true (`self.Left`) :!label _label)
                    (set `self.isReservingOther` true)
                    (bind (_direction _postion_alpha) (`Timeline|Move Left` :!via `PlayFromStart`)
                      (:`Update`
                        (`self.K2_SetActorLocation` (`self.Item Held`) (`KismetMathLibrary.VLerp` (`SceneComponent.K2_GetComponentLocation` (`self.Scene`)) (`SceneComponent.K2_GetComponentLocation` (`/Game/Blueprints/BP_Container.Scene` (`self.Left`))) _postion_alpha) false false))
                      (:`Finished`
                        (bind _success (`/Game/BPI/BPI_Interact.Deposit` _left (`self.Item Held`)))
                        (if _success
                          (set `/Game/Blueprints/BP_Container.Reserved` false _left)
                          (set `self.isReservingOther` false)
                          (set `self.HasItem` false)
                          (set `self.Item Held` null)))))))))
          (else
            (goto _label))))
      (:`NewEnumerator4`
        ;[1 1 1] Destination Occupied
        (if (or (`/Game/Blueprints/BP_Container.HasItem` _right_2) (`/Game/Blueprints/BP_Container.Reserved` _right_2))
          ;[1 1 1] Check Again Loop
          (`Timeline|Check Right` :!via `PlayFromStart`
            (:`Check`
              (if (not (or (`/Game/Blueprints/BP_Container.HasItem` _right) (`/Game/Blueprints/BP_Container.Reserved` _right)))
                (`|ExecutionSequence`
                  (:`then_0`
                    (`TimelineComponent.Stop` (`self.Check Right`)))
                  (:`then_1`
                    ;[1 1 1] Move Item
                    (set `/Game/Blueprints/BP_Container.Reserved` true (`self.Right`) :!label _label_2)
                    (set `self.isReservingOther` true)
                    (bind (_direction_2 _postion_alpha_2) (`Timeline|Move Right` :!via `PlayFromStart`)
                      (:`Update`
                        (`self.K2_SetActorLocation` (`self.Item Held`) (`KismetMathLibrary.VLerp` (`SceneComponent.K2_GetComponentLocation` (`self.Scene`)) (`SceneComponent.K2_GetComponentLocation` (`/Game/Blueprints/BP_Container.Scene` (`self.Right`))) _postion_alpha_2) false false))
                      (:`Finished`
                        (bind _success_2 (`/Game/BPI/BPI_Interact.Deposit` _right_3 (`self.Item Held`)))
                        (if _success_2
                          (set `/Game/Blueprints/BP_Container.Reserved` false _right_3)
                          (set `self.isReservingOther` false)
                          (set `self.HasItem` false)
                          (set `self.Item Held` null)))))))))
          (else
            (goto _label_2))))
      (:`NewEnumerator5`
        ;[1 1 1] Destination Occupied
        (if (or (`/Game/Blueprints/BP_Container.HasItem` _forward_2) (`/Game/Blueprints/BP_Container.Reserved` _forward_2))
          ;[1 1 1] Check Again Loop
          (`Timeline|Check Front` :!via `PlayFromStart`
            (:`Check`
              (if (not (or (`/Game/Blueprints/BP_Container.HasItem` _forward_3) (`/Game/Blueprints/BP_Container.Reserved` _forward_3)))
                (`|ExecutionSequence`
                  (:`then_0`
                    (`TimelineComponent.Stop` (`self.Check Front`)))
                  (:`then_1`
                    ;[1 1 1] Move Item
                    (set `/Game/Blueprints/BP_Container.Reserved` true (`self.Forward`) :!label _label_3)
                    (set `self.isReservingOther` true)
                    (bind (_direction_3 _postion_alpha_3) (`Timeline|Move Forward` :!via `PlayFromStart`)
                      (:`Update`
                        (`self.K2_SetActorLocation` (`self.Item Held`) (`KismetMathLibrary.VLerp` (`SceneComponent.K2_GetComponentLocation` (`self.Scene`)) (`SceneComponent.K2_GetComponentLocation` (`/Game/Blueprints/BP_Container.Scene` (`self.Forward`))) _postion_alpha_3) false false))
                      (:`Finished`
                        (bind _success_3 (`/Game/BPI/BPI_Interact.Deposit` _forward (`self.Item Held`)))
                        (if _success_3
                          (set `/Game/Blueprints/BP_Container.Reserved` false _forward)
                          (set `self.isReservingOther` false)
                          (set `self.HasItem` false)
                          (set `self.Item Held` null)))))))))
          (else
            (goto _label_3)))))))

(fn `Change Colour`
  (params (Side :type "/Game/Core/ESide Enum" :default "NewEnumerator0"))
  (bind _m_0 (`self.M_0`))
  (bind (_output_side _output_colour) (break `/Game/Core/FSorterColour` (`|GetArrayItem` _m_0 1)))
  (bind (_output_side_2 _output_colour_2) (break `/Game/Core/FSorterColour` (`|GetArrayItem` _m_0 2)))
  (bind (_output_side_3 _output_colour_3) (break `/Game/Core/FSorterColour` (`|GetArrayItem` _m_0 3)))
  (bind (_output_side_4 _output_colour_4) (break `/Game/Core/FSorterColour` (`|GetArrayItem` _m_0)))
  (bind _returnvalue (select `/Game/Core/EColour` (select `/Game/Core/ESide` Side :`NewEnumerator0` "NewEnumerator0" :`NewEnumerator1` "NewEnumerator0" :`NewEnumerator2` "NewEnumerator0" :`NewEnumerator3` _output_colour_2 :`NewEnumerator4` _output_colour_3 :`NewEnumerator5` _output_colour_4 :`NewEnumerator6` _output_colour) :`NewEnumerator0` "NewEnumerator1" :`NewEnumerator1` "NewEnumerator2" :`NewEnumerator2` "NewEnumerator4" :`NewEnumerator4` "NewEnumerator0" :!type "/Game/Core/EColour Enum"))
  (switch `/Game/Core/ESide` Side
    (:`NewEnumerator3`
      (set `self.Left Colour` _returnvalue))
    (:`NewEnumerator4`
      (set `self.Right Colour` _returnvalue))
    (:`NewEnumerator5`
      (set `self.Foward Colour` _returnvalue))
    (:`NewEnumerator6`
      (set `self.Back Colour` _returnvalue)))
  (`self.Set Mesh Colour`))

(fn `Get Neighbour`
  (bind _staticmeshcomponent (`self.StaticMeshComponent`))
  (bind _staticmeshcomponent_2 (`self.StaticMeshComponent`))
  (bind _staticmeshcomponent_3 (`self.StaticMeshComponent`))
  (bind _staticmeshcomponent_4 (`self.StaticMeshComponent`))
  (bind _returnvalue (`SceneComponent.K2_GetComponentLocation` _staticmeshcomponent_3))
  (bind _returnvalue_2 (`SceneComponent.K2_GetComponentLocation` _staticmeshcomponent_4))
  (bind _returnvalue_3 (`SceneComponent.K2_GetComponentLocation` _staticmeshcomponent))
  (bind _returnvalue_4 (`SceneComponent.K2_GetComponentLocation` _staticmeshcomponent_2))
  (bind _outhit (`KismetSystemLibrary.LineTraceSingle` (+ _returnvalue_4 (0.0 0.0 10.0)) (+ (+ _returnvalue_4 (* (`KismetMathLibrary.GetForwardVector` (`SceneComponent.K2_GetComponentRotation` _staticmeshcomponent_2)) 100.0)) (0.0 0.0 10.0)) "TraceTypeQuery1"))
  (bind _asbp_container (cast `/Game/Blueprints/BP_Container` (`.HitActor` (`GameplayStatics.BreakHitResult` _outhit)))
    (:`then`
      (set `self.Has Forward Destination` true)
      (set `self.Forward` _asbp_container))
    (:`CastFailed`
      (set `self.Has Forward Destination` false)
      (set `self.Forward` null)))
  (bind _outhit_2 (`KismetSystemLibrary.LineTraceSingle` (+ _returnvalue_2 (0.0 0.0 10.0)) (+ (- _returnvalue_2 (* (`KismetMathLibrary.GetForwardVector` (`SceneComponent.K2_GetComponentRotation` _staticmeshcomponent_4)) 100.0)) (0.0 0.0 10.0)) "TraceTypeQuery1"))
  (bind _asbp_container_2 (cast `/Game/Blueprints/BP_Container` (`.HitActor` (`GameplayStatics.BreakHitResult` _outhit_2)))
    (:`then`
      (set `self.Has Back Destination` true)
      (set `self.Back` _asbp_container_2))
    (:`CastFailed`
      (set `self.Has Back Destination` false)
      (set `self.Back` null)))
  (bind _outhit_3 (`KismetSystemLibrary.LineTraceSingle` (+ _returnvalue (0.0 0.0 10.0)) (+ (+ _returnvalue (* (`KismetMathLibrary.GetRightVector` (`SceneComponent.K2_GetComponentRotation` _staticmeshcomponent_3)) 100.0)) (0.0 0.0 10.0)) "TraceTypeQuery1"))
  (bind _asbp_container_3 (cast `/Game/Blueprints/BP_Container` (`.HitActor` (`GameplayStatics.BreakHitResult` _outhit_3)))
    (:`then`
      (set `self.Has Right Destination` true)
      (set `self.Right` _asbp_container_3))
    (:`CastFailed`
      (set `self.Has Right Destination` false)
      (set `self.Right` null)))
  (bind _outhit_4 (`KismetSystemLibrary.LineTraceSingle` (+ _returnvalue_3 (0.0 0.0 10.0)) (+ (- _returnvalue_3 (* (`KismetMathLibrary.GetRightVector` (`SceneComponent.K2_GetComponentRotation` _staticmeshcomponent)) 100.0)) (0.0 0.0 10.0)) "TraceTypeQuery1"))
  (bind _asbp_container_4 (cast `/Game/Blueprints/BP_Container` (`.HitActor` (`GameplayStatics.BreakHitResult` _outhit_4)))
    (:`then`
      (set `self.Has Left Destination` true)
      (set `self.Left` _asbp_container_4))
    (:`CastFailed`
      (set `self.Has Left Destination` false)
      (set `self.Left` null))))

(fn `Sort`
  (params (`Tray Colour` :type "/Game/Core/EColour Enum" :default "NewEnumerator0"))
  (returns (`Out Side` :type "/Game/Core/ESide Enum"))
  (locals (Side :type "Array of /Game/Core/ESide Enum") (Colour :type "Array of /Game/Core/EColour Enum") (`Array Index` :type Integer :default 0))
  (bind _m_0 (`self.M_0`))
  (bind _array_index (`local.Array Index`))
  (bind _output_side (break `/Game/Core/FSorterColour` (`|GetArrayItem` _m_0 (`KismetArrayLibrary.Array_LastIndex` _m_0))))
  (for _array_element (`self.M_0`)
    (bind (_side _colour) (break `/Game/Core/FSorterColour` _array_element))
    (`KismetArrayLibrary.Array_Add` (`local.Side`) _side)
    (`KismetArrayLibrary.Array_Add` (`local.Colour`) _colour))
  (bind _output_get (set `local.Array Index` (`KismetArrayLibrary.Array_Find` (`local.Colour`) `Tray Colour`)))
  (if (not (>= _output_get 0))
    (bind _output_get_2 (set `local.Array Index` (`KismetArrayLibrary.Array_Find` (`local.Colour`) "NewEnumerator0")))
    (if (>= _output_get_2 0)
      _
      (else
        (return "NewEnumerator0"))))
  (`KismetArrayLibrary.Array_Add` _m_0 (make `/Game/Core/FSorterColour` (`|GetArrayItem` (`local.Side`) _array_index) (`|GetArrayItem` (`local.Colour`) _array_index)))
  (`KismetArrayLibrary.Array_Remove` _m_0 (`local.Array Index`))
  (return _output_side))

(fn `UserConstructionScript`
  (bind _staticmeshcomponent (`self.StaticMeshComponent`))
  (bind _m_0 (`self.M_0`))
  (bind (_output_side _output_colour) (break `/Game/Core/FSorterColour` (`|GetArrayItem` _m_0 1)))
  (bind (_output_side_2 _output_colour_2) (break `/Game/Core/FSorterColour` (`|GetArrayItem` _m_0 2)))
  (bind (_output_side_3 _output_colour_3) (break `/Game/Core/FSorterColour` (`|GetArrayItem` _m_0 3)))
  (bind (_output_side_4 _output_colour_4) (break `/Game/Core/FSorterColour` (`|GetArrayItem` _m_0)))
  (`parent.UserConstructionScript`)
  (`PrimitiveComponent.SetMaterial` _staticmeshcomponent 1 (select `/Game/Core/EColour` _output_colour :`NewEnumerator0` "/Game/Materials/Sorter/M_Sorter_Conveyor_None.M_Sorter_Conveyor_None" :`NewEnumerator1` "/Game/Materials/Sorter/M_Sorter_Conveyor_Red.M_Sorter_Conveyor_Red" :`NewEnumerator2` "/Game/Materials/Sorter/M_Sorter_Conveyor_Green.M_Sorter_Conveyor_Green" :`NewEnumerator4` "/Game/Materials/Sorter/M_Sorter_Conveyor_Blue.M_Sorter_Conveyor_Blue" :!type "MaterialInstance Object Reference"))
  (`PrimitiveComponent.SetMaterial` _staticmeshcomponent 3 (select `/Game/Core/EColour` _output_colour_3 :`NewEnumerator0` "/Game/Materials/Sorter/M_Sorter_Conveyor_None.M_Sorter_Conveyor_None" :`NewEnumerator1` "/Game/Materials/Sorter/M_Sorter_Conveyor_Red.M_Sorter_Conveyor_Red" :`NewEnumerator2` "/Game/Materials/Sorter/M_Sorter_Conveyor_Green.M_Sorter_Conveyor_Green" :`NewEnumerator4` "/Game/Materials/Sorter/M_Sorter_Conveyor_Blue.M_Sorter_Conveyor_Blue" :!type "MaterialInstance Object Reference"))
  (`PrimitiveComponent.SetMaterial` _staticmeshcomponent 4 (select `/Game/Core/EColour` _output_colour_4 :`NewEnumerator0` "/Game/Materials/Sorter/M_Sorter_Conveyor_None.M_Sorter_Conveyor_None" :`NewEnumerator1` "/Game/Materials/Sorter/M_Sorter_Conveyor_Red.M_Sorter_Conveyor_Red" :`NewEnumerator2` "/Game/Materials/Sorter/M_Sorter_Conveyor_Green.M_Sorter_Conveyor_Green" :`NewEnumerator4` "/Game/Materials/Sorter/M_Sorter_Conveyor_Blue.M_Sorter_Conveyor_Blue" :!type "MaterialInstance Object Reference"))
  (`PrimitiveComponent.SetMaterial` _staticmeshcomponent 2 (select `/Game/Core/EColour` _output_colour_2 :`NewEnumerator0` "/Game/Materials/Sorter/M_Sorter_Conveyor_None.M_Sorter_Conveyor_None" :`NewEnumerator1` "/Game/Materials/Sorter/M_Sorter_Conveyor_Red.M_Sorter_Conveyor_Red" :`NewEnumerator2` "/Game/Materials/Sorter/M_Sorter_Conveyor_Green.M_Sorter_Conveyor_Green" :`NewEnumerator4` "/Game/Materials/Sorter/M_Sorter_Conveyor_Blue.M_Sorter_Conveyor_Blue" :!type "MaterialInstance Object Reference")))

(fn `Withdraw`
  (returns (Item :type "/Game/Blueprints/Parts/BP_Part Object Reference") (Success :type Boolean))
  (bind _printdebugs (`self.PrintDebugs`))
  (if (`self.HasItem`)
    (`KismetSystemLibrary.PrintString` "Withdraw Success" _printdebugs _printdebugs)
    (set `self.HasItem` false)
    (`TimelineComponent.Stop` (`self.Check Front`))
    (`TimelineComponent.Stop` (`self.Move Forward`))
    (`TimelineComponent.Stop` (`self.Move Right`))
    (`TimelineComponent.Stop` (`self.Move Left`))
    (`TimelineComponent.Stop` (`self.Check Left`))
    (`TimelineComponent.Stop` (`self.Check Right`))
    (`self.Item Changed` "NewEnumerator1")
    (if (`self.isReservingOther`)
      (set `/Game/Blueprints/BP_Container.Reserved` false (`self.Forward`)))
    (return (`self.Item Held`) true)
    (else
      (`KismetSystemLibrary.PrintString` "Withdraw Fail" _printdebugs _printdebugs)
      (return null false))))