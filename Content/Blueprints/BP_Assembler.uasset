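; Factory assembler with a robot arm that moves its held item onto the item in the container in front of it and combines the two.
; A forward line trace at BeginPlay finds the destination BP_Container.
; ItemChanged uses a CheckAgain timeline to wait until the destination holds an unreserved, combinable item, then reserves it.
; An arm timeline drives four joint rotations, with event tracks for pickup and drop-off; the older MoveAlong lerp is unconnected.
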(event `self.ReceiveBeginPlay`
  (`parent.ReceiveBeginPlay`)
  (`self.Get Neighbour`))

(event `self.Item Changed`
  (params (`Change Type` :type "/Game/Core/EItemChange Enum" :default "NewEnumerator0"))
  (bind _destination (`self.Destination`))
  (bind _destination_2 (`self.Destination`))
  (bind _destination_3 (`self.Destination`))
  ;[1 1 1] Has Item And Valid Destination
  (if (and (`self.Has Destination`) (`self.HasItem`))
    ;[1 1 1] Destination Is Reserved or Empty
    (if (or (not (`/Game/Blueprints/BP_Container.HasItem` _destination_2)) (`/Game/Blueprints/BP_Container.Reserved` _destination_2))
      ;[1 1 1] Check Again Loop
      (`Timeline|Check Again` :!via `PlayFromStart`
        (:`Check`
          (if (not (or (not (`/Game/Blueprints/BP_Container.HasItem` _destination_3)) (`/Game/Blueprints/BP_Container.Reserved` _destination_3)))
            ;[1 1 1] Can Combine Items?
            (bind _success (`/Game/Blueprints/Parts/BP_Part.Combine` (`/Game/Blueprints/BP_Container.Item Held` (`self.Destination`)) (`self.Item Held`) true))
            (if _success
              (`|ExecutionSequence` :!label _label
                (:`then_0`
                  (`TimelineComponent.Stop` (`self.Check Again`)))
                (:`then_1`
                  (set `/Game/Blueprints/BP_Container.Reserved` true (`self.Destination`))
                  (set `self.isReservingOther` true)
                  (bind (_direction _section_0 _section_1 _section_2 _section_3) (`Timeline|Timeline_0` :!via `PlayFromStart`)
                    (:`Update`
                      (`SceneComponent.K2_SetRelativeRotation` (`self.RobotArm_Section_0`) (`KismetMathLibrary.MakeRotator` 0.0 0.0 _section_0) false false)
                      (`SceneComponent.K2_SetRelativeRotation` (`self.RobotArm_Section_1`) (`KismetMathLibrary.MakeRotator` _section_1) false false)
                      (`SceneComponent.K2_SetRelativeRotation` (`self.RobotArm_Section_2`) (`KismetMathLibrary.MakeRotator` _section_2) false false)
                      (`SceneComponent.K2_SetRelativeRotation` (`self.RobotArm_Section_3`) (`KismetMathLibrary.MakeRotator` _section_3) false false))
                    (:`Finished`
                      (set `self.isReservingOther` false)
                      (set `self.HasItem` false)
                      (set `self.Item Held` null))
                    (:`Pickup`
                      (`self.K2_AttachToComponent` (`self.Item Held`) (`self.Grab`) "None" "SnapToTarget" "SnapToTarget" "SnapToTarget" true))
                    (:`Drop Off`
                      (bind _success_2 (`/Game/Blueprints/Parts/BP_Part.Combine` (`/Game/Blueprints/BP_Container.Item Held` _destination) (`self.Item Held`) false))
                      (if _success_2
                        (set `/Game/Blueprints/BP_Container.Reserved` false _destination))))))))))
      (else
        (bind _success_3 (`/Game/Blueprints/Parts/BP_Part.Combine` (`/Game/Blueprints/BP_Container.Item Held` (`self.Destination`)) (`self.Item Held`) true))
        (if _success_3
          (goto _label)
          (else
            (`TimelineComponent.PlayFromStart` (`self.Check Again`))))))))

(fn `Get Neighbour`
  (bind _staticmeshcomponent (`self.StaticMeshComponent`))
  (bind _returnvalue (`SceneComponent.K2_GetComponentLocation` _staticmeshcomponent))
  (bind _outhit (`KismetSystemLibrary.LineTraceSingle` :`Start` (+ _returnvalue (0.0 0.0 10.0)) :`End` (+ (+ _returnvalue (* (`KismetMathLibrary.GetForwardVector` (`SceneComponent.K2_GetComponentRotation` _staticmeshcomponent)) 100.0)) (0.0 0.0 10.0)) :`TraceChannel` "TraceTypeQuery1" :`DrawDebugType` "Persistent"))
  (bind _asbp_container (cast `/Game/Blueprints/BP_Container` (`.HitActor` (`GameplayStatics.BreakHitResult` _outhit)))
    (:`then`
      (set `self.Has Destination` true)
      (set `self.Destination` _asbp_container))
    (:`CastFailed`
      (set `self.Has Destination` false)
      (set `self.Destination` null))))

(fn `UserConstructionScript`
  (`parent.UserConstructionScript`))