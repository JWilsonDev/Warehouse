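; Craftable furniture part that accepts other parts into named slots and tracks its furniture type, colour, material and stage.
; Combine matches an item by part name, in list order or any order, with an optional check-only mode.
; A successful combine copies the item's mesh onto the socket, removes the slot, destroys the item and advances the stage.
; Helpers recolour all meshes through dynamic materials, show a coloured tray or apply a ghost material.
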(fn `Combine`
  (params (Item :type "/Game/Blueprints/Parts/BP_Part Object Reference") (`Check Only` :type Boolean))
  (returns (Success :type Boolean))
  (locals (`New Part Name` :type "/Game/Core/EParts Enum" :default "NewEnumerator0") (`Compatible Slots` :type "Array of Integer"))
  (bind _mesh (`/Game/Blueprints/Parts/BP_Part.Mesh` (`local.Item`)))
  (if (> (`KismetArrayLibrary.Array_Length` (`self.Parts`)) 0)
    (set `local.New Part Name` (`/Game/Blueprints/Parts/BP_Part.Part Name` Item))
    (if (`self.Ordered Crafting`)
      (if (`|EnumEquality` (`.PartName_5_8ADDF614461E7FC47908A08FE2860EDF` (break `/Game/Core/FPartSlotDic` (`|GetArrayItem` (`self.Parts`)))) (`local.New Part Name`))
        (`KismetArrayLibrary.Array_Add` (`local.Compatible Slots`))
        (if (`local.Check Only`)
          (return true)
          (else
            _))
        (else
          (return false)))
      (else
        (for (_array_element _array_index) (`self.Parts`)
          (if (`|EnumEquality` (`.PartName_5_8ADDF614461E7FC47908A08FE2860EDF` (break `/Game/Core/FPartSlotDic` _array_element)) (`local.New Part Name`))
            (`KismetArrayLibrary.Array_Add` (`local.Compatible Slots`) _array_index)))
        (if (> (`KismetArrayLibrary.Array_Length` (`local.Compatible Slots`)) 0)
          (if (`local.Check Only`)
            (return true)
            (else
              _))
          (else
            (return false)))))
    (bind _returnvalue (`AddComponent|NODE_AddStaticMeshComponent-0`))
    (`StaticMeshComponent.SetStaticMesh` _returnvalue (`StaticMeshComponent.StaticMesh` _mesh))
    (`KismetArrayLibrary.Array_Add` (`self.Meshes`) _returnvalue)
    (`PrimitiveComponent.SetMaterial` _returnvalue 0 (`PrimitiveComponent.GetMaterial` _mesh 0))
    (bind _returnvalue_2 (`SceneComponent.K2_AttachToComponent` _returnvalue (`self.Mesh`) (`.SlotName_6_BE0F1137472307EBC27F3885AF18CF49` (break `/Game/Core/FPartSlotDic` (`|GetArrayItem` (`self.Parts`) (`|GetArrayItem` (`local.Compatible Slots`))))) "SnapToTarget" "SnapToTarget" "SnapToTarget" true))
    (if _returnvalue_2
      (`KismetArrayLibrary.Array_Remove` (`self.Parts`) (`|GetArrayItem` (`local.Compatible Slots`)))
      (`self.K2_DestroyActor` (`local.Item`))
      (bind _result (`/Engine/EditorBlueprintResources/StandardMacros.IncrementInt` (`self.Stage`))
        (:`  `
          (`self.DKWhatToCallThisYet` _result)))
      (else
        (`KismetSystemLibrary.PrintString` (`KismetStringLibrary.Concat_StrStr` (`KismetSystemLibrary.GetClassDisplayName` (`GameplayStatics.GetObjectClass` self)) " Contains Invalid Slot Name: "))))
    (return _returnvalue_2)))

(fn `DKWhatToCallThisYet`
  (params (Stage :type Integer))
  (bind (_furniturestructure_finaltype _furniturestructure_currenttype _furniturestructure_colour _furniturestructure_material) (break `/Game/Core/FFurniture` (`self.FurnitureStructure`)))
  (set `self.FurnitureStructure` (make `/Game/Core/FFurniture` _furniturestructure_finaltype _furniturestructure_currenttype _furniturestructure_colour _furniturestructure_material Stage))
  (if (== Stage 1)
    (`self.Update Part Status` "NewEnumerator0")))

(fn `Set Item As Filter`
  (for _array_element (`self.Meshes`)
    (`PrimitiveComponent.SetMaterial` _array_element 0 "/Game/Materials/M_Ghost.M_Ghost")))

(fn `Set Tray Filter`
  (params (`Active?` :type Boolean) (Colour :type "/Game/Core/EColour Enum" :default "NewEnumerator0"))
  (bind _tray (`self.Tray`))
  (if `Active?`
    (bind _output_get (set `self.Tray Colour` Colour))
    (`PrimitiveComponent.SetMaterial` _tray 0 (select `/Game/Core/EColour` _output_get :`NewEnumerator1` "/Game/Materials/Filter/M_Tray_Red.M_Tray_Red" :`NewEnumerator2` "/Game/Materials/Filter/M_Tray_Green.M_Tray_Green" :`NewEnumerator4` "/Game/Materials/Filter/M_Tray_Blue.M_Tray_Blue" :!type "MaterialInterface Object Reference"))
    (`SceneComponent.SetVisibility` _tray true false)
    (else
      (`SceneComponent.SetVisibility` (`self.Tray`) false false))))

(fn `Update Part Colour`
  (params (Colour :type "/Game/Core/EColour Enum" :default "NewEnumerator0"))
  (bind (_finaltype _currenttype _colour _material _stage) (break `/Game/Core/FFurniture` (`self.FurnitureStructure`)))
  (set `self.FurnitureStructure` (make `/Game/Core/FFurniture` _finaltype _currenttype Colour _material _stage))
  (for _array_element (`self.Meshes`)
    (bind _returnvalue (`PrimitiveComponent.CreateDynamicMaterialInstance` _array_element 0 (`PrimitiveComponent.GetMaterial` _array_element 0) "None"))
    (`MaterialInstanceDynamic.SetVectorParameterValue` _returnvalue "Colour" (select `/Game/Core/EColour` Colour :`NewEnumerator1` (struct :`R` 1.0 :`A` 1.0) :`NewEnumerator2` (struct :`G` 1.0 :`A` 1.0) :`NewEnumerator4` (struct :`B` 1.0 :`A` 1.0) :!type "LinearColor Structure"))))

(fn `Update Part Status`
  (params (FurnitureType :type "/Game/Core/EFurniture Enum" :default "NewEnumerator3"))
  (bind (_finaltype _currenttype _colour _material _stage) (break `/Game/Core/FFurniture` (`self.FurnitureStructure`)))
  (set `self.FurnitureStructure` (make `/Game/Core/FFurniture` _finaltype FurnitureType _colour _material _stage)))

(fn `UserConstructionScript`
  (`KismetArrayLibrary.Array_Add` (`self.Meshes`) (`self.Mesh`)))