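; Chair seat part for furniture assembly, a child Blueprint that builds on its parent's combine and stage logic.
; Combine defers to the parent; older code that snaps leg and back meshes onto sockets and destroys the source items is left disconnected.
; DKWhatToCallThisYet runs the parent, then raises the seat mesh and updates FurnitureStatus at stage 4, and advances the status again at stage 5.
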(fn `Combine`
  (params (Item :type "/Game/Blueprints/Parts/BP_Part Object Reference"))
  (returns (Success :type Boolean))
  (bind _success (`parent.Combine` Item))
  (return _success))

(fn `DKWhatToCallThisYet`
  (params (Stage :type Integer))
  (`parent.DKWhatToCallThisYet` Stage)
  (switch `int` Stage
    (:`4`
      (`SceneComponent.K2_SetRelativeLocationAndRotation` :`self` (`self.Mesh`) :`NewLocation` (0.0 0.0 25.0))
      (set `self.Furniture Status` "NewEnumerator1"))
    (:`5`
      (set `self.Furniture Status` "NewEnumerator2"))))

(fn `UserConstructionScript`
  (`parent.UserConstructionScript`))