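; BP_Supply is a supply source actor that dispenses and takes back a single configured item type.
; Withdraw always spawns a new StockItem at the SpawnPoint transform and returns it as a success, so stock is unlimited.
; Deposit destroys the passed item and returns true only if its class exactly matches StockItem, otherwise it returns false.
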(event `self.ReceiveTick`
  (params (DeltaSeconds :type "Float (single-precision)"))
  (`parent.ReceiveTick` DeltaSeconds))

(fn `Deposit`
  (params (Item :type "/Game/Blueprints/Parts/BP_Part Object Reference"))
  (returns (Success :type Boolean))
  (if (== (`GameplayStatics.GetObjectClass` Item) (`self.Stock Item`))
    (`self.K2_DestroyActor` (`local.Item`))
    (return true)
    (else
      (return false))))

(fn `UserConstructionScript`
  (`parent.UserConstructionScript`))

(fn `Withdraw`
  (returns (Item :type "/Game/Blueprints/Parts/BP_Part Object Reference") (Success :type Boolean))
  (bind _returnvalue (`|SpawnActorFromClass` (`self.Stock Item`) (`SceneComponent.K2_GetComponentToWorld` (`self.SpawnPoint`)) "AlwaysSpawn" "OverrideRootScale" null null))
  (return _returnvalue true))