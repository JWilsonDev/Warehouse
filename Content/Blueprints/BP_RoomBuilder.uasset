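; BP_RoomBuilder procedurally builds a rectangular tiled room in its Construction Script from Width and Length.
; It fills a FloorTiles grid, then adds a floor instance per tile at 100-unit spacing.
; Each tile checks its four neighbors against that array and places rotated wall instances on open edges, using ShortWall for the -X side.
; Walls and Floor instances are cleared on each rebuild, but ShortWall is not.
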(fn `UserConstructionScript`
  (bind _floor_tiles (`self.Floor Tiles`))
  (`InstancedStaticMeshComponent.ClearInstances` (`self.Walls`))
  (`InstancedStaticMeshComponent.ClearInstances` (`self.Floor`))
  (`KismetArrayLibrary.Array_Clear` (`self.Floor Tiles`))
  (for _index (range (`self.Width`))
    (for _index_2 (range (`self.Length`))
      (`KismetArrayLibrary.Array_Add` (`self.Floor Tiles`) (make `IntVector` _index_2 _index))))
  (for _array_element _floor_tiles
    (bind (_x _y) (break `IntVector` _array_element))
    (`InstancedStaticMeshComponent.AddInstance` (`self.Floor`) (`KismetMathLibrary.MakeTransform` (* (`KismetMathLibrary.MakeVector` (`KismetMathLibrary.Conv_IntToDouble` _x) (`KismetMathLibrary.Conv_IntToDouble` _y)) 100)) false)
    ;[1 1 1] Spawn Walls
    (for _index_3 (range 4)
      (if (not (select `int` _index_3 :`0` (`.IsInArray` (`self.TestRelativeTileLocation` _array_element _floor_tiles 1)) :`1` (`.IsInArray` (`self.TestRelativeTileLocation` _array_element _floor_tiles 0 1)) :`2` (`.IsInArray` (`self.TestRelativeTileLocation` _array_element _floor_tiles -1)) :`3` (`.IsInArray` (`self.TestRelativeTileLocation` _array_element _floor_tiles 0 -1))))
        (if (== _index_3 2)
          (bind _returnvalue (* (`KismetMathLibrary.Conv_IntVectorToVector` _array_element) 100.0))
          (bind _returnvalue_2 (select `int` _index_3 :`0` (struct :`Yaw` 90.0) :`1` (struct :`Yaw` 180.0) :`2` (struct :`Yaw` -90.0) :`3` (struct) :!type "Rotator Structure"))
          (`InstancedStaticMeshComponent.AddInstance` (`self.ShortWall`) (`KismetMathLibrary.MakeTransform` _returnvalue _returnvalue_2) false)
          (else
            (`InstancedStaticMeshComponent.AddInstance` (`self.Walls`) (`KismetMathLibrary.MakeTransform` _returnvalue _returnvalue_2) false)))))))