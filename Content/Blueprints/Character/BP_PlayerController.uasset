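; BP_PlayerController is a player controller that turns movement axis input into movement of the player character.
; On BeginPlay it casts the controlled pawn to BP_Player and stores it as PlayerCharacter.
; The Move Forward and Move Right axis events add movement input to that character along the forward and right vectors of the full control rotation, without isolating yaw.
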(event `self.ReceiveBeginPlay`
  (set `self.Player Character` (cast `/Game/Blueprints/Character/BP_Player` (`self.K2_GetPawn`) :!pure true)))

(event `InputAxis|Move Forward`
  (params (AxisValue :type "Float (single-precision)"))
  (`Pawn.AddMovementInput` (`self.Player Character`) (`KismetMathLibrary.GetForwardVector` (`self.GetControlRotation`)) AxisValue false))

(event `InputAxis|Move Right`
  (params (AxisValue :type "Float (single-precision)"))
  (`Pawn.AddMovementInput` (`self.Player Character`) (`KismetMathLibrary.GetRightVector` (`self.GetControlRotation`)) AxisValue false))

(fn `UserConstructionScript`)