(event `InputAction|Jump`
  (params (Key :type "Key Structure"))
  ;[1 1 1] Player Movement
  (:`Pressed`
    (`self.Jump`)))

(event `InputAxis|Move Forward`
  (params (AxisValue :type "Float (single-precision)"))
  ;[1 1 1] Player Movement
  (`self.AddMovementInput` (`KismetMathLibrary.GetForwardVector` (`self.GetControlRotation`)) AxisValue))

(event `InputAxis|Move Right`
  (params (AxisValue :type "Float (single-precision)"))
  ;[1 1 1] Player Movement
  (`self.AddMovementInput` (`KismetMathLibrary.GetRightVector` (`self.GetControlRotation`)) AxisValue))

(event `self.ReceiveTick`
  (params (DeltaSeconds :type "Float (single-precision)"))
  ;[1 1 1] Tick
  (`self.Linetrace`)
  (`self.Snap Check`))

(event `InputAction|Primary Action`
  (params (Key :type "Key Structure"))
  (bind _looking_at (`self.Looking At`))
  ;[1 1 1] Basic Interaction
  (:`Pressed`
    (if (`|EnumEquality` (`self.Mode`) "NewEnumerator0")
      (`/Engine/EditorBlueprintResources/StandardMacros.IsValid` (`self.Looking At`)
        (:`Is Valid`
          (if (`self.Has Item`)
            (if (not (`/Game/Blueprints/BP_Container.Reserved` _looking_at))
              (bind _success (`/Game/BPI/BPI_Interact.Deposit` _looking_at (`self.Item Held`)))
              (if _success
                (set `self.Has Item` false)
                (set `self.Item Held` null)))
            (else
              (bind (_item _success_2) (`/Game/BPI/BPI_Interact.Withdraw` (`self.Looking At`)))
              (if _success_2
                (set `self.Has Item` true)
                (`self.K2_DetachFromActor` _item "KeepWorld" "KeepWorld" "KeepWorld")
                (bind _output_get (set `self.Item Held` _item))
                (`self.K2_AttachToComponent` _output_get (`self.ItemPoint`) "None" "SnapToTarget" "SnapToTarget" "SnapToTarget" true)))))))))

(event `InputAction|Primary Action`
  (params (Key :type "Key Structure"))
  (bind (_newvar_0_location _newvar_0_rotation _newvar_0_scale) (`KismetMathLibrary.BreakTransform` (`self.NewVar_0`)))
  (bind _looking_at (`self.Looking At`))
  (bind _looking_at_2 (`self.Looking At`))
  (bind (_newvar_0_location_2 _newvar_0_rotation_2 _newvar_0_scale_2) (`KismetMathLibrary.BreakTransform` (`self.NewVar_0`)))
  (:`Pressed`
    (if (`|EnumEquality` (`self.Mode`) "NewEnumerator1")
      (`/Engine/EditorBlueprintResources/StandardMacros.IsValid` (`self.Looking At`)
        (:`Is Valid`
          (if (`self.Has Container`)
            (`KismetSystemLibrary.PrintString` "Swap Containers")
            (`self.K2_DestroyActor` (`self.Container Held`))
            (bind _output_get (set `self.Old Held Container` (`self.Held Container`)))
            (set `self.Held Container` (`GameplayStatics.GetObjectClass` (`self.Looking At`)))
            (`|SpawnActorFromClass` _output_get (`self.NewVar_0`) "AlwaysSpawn" "OverrideRootScale" null false "0.000000,0.000000,0.000000|0.000000,0.000000,-0.000000|1.000000,1.000000,1.000000" null)
            (set `self.Container Held` null)
            (set `self.NewVar_0` (`self.GetTransform` _looking_at))
            (`self.K2_DestroyActor` _looking_at)
            (bind _returnvalue (`|SpawnActorFromClass` (`self.Held Container`) (`KismetMathLibrary.MakeTransform` (`self.Round To Grid` _newvar_0_location) _newvar_0_rotation _newvar_0_scale) "AlwaysSpawn" "OverrideRootScale" null true "0.000000,0.000000,0.000000|0.000000,0.000000,-0.000000|1.000000,1.000000,1.000000" null))
            (set `self.Container Held` _returnvalue)
            (set `self.Has Container` true)
            (else
              (bind _output_get_2 (set `self.Held Container` (`GameplayStatics.GetObjectClass` _looking_at_2)))
              (set `self.NewVar_0` (`self.GetTransform` _looking_at_2))
              (`self.K2_DestroyActor` _looking_at_2)
              (bind _returnvalue_2 (`|SpawnActorFromClass` _output_get_2 (`KismetMathLibrary.MakeTransform` (`self.Round To Grid` _newvar_0_location_2) _newvar_0_rotation_2 _newvar_0_scale_2) "AlwaysSpawn" "OverrideRootScale" null true "0.000000,0.000000,0.000000|0.000000,0.000000,-0.000000|1.000000,1.000000,1.000000" null))
              (set `self.Container Held` _returnvalue_2)
              (set `self.Has Container` true))))
        (:`Is Not Valid`
          (if (`self.Has Container`)
            (`KismetSystemLibrary.PrintString` "Attempt Place")
            (`self.K2_DestroyActor` (`self.Container Held`))
            (`|SpawnActorFromClass` (`self.Held Container`) (`self.NewVar_0`) "AlwaysSpawn" "OverrideRootScale" null false "0.000000,0.000000,0.000000|0.000000,0.000000,-0.000000|1.000000,1.000000,1.000000" null)
            (set `self.Has Container` false)
            (set `self.Container Held` null)
            (else
              (`KismetSystemLibrary.PrintString` "Do Nothing"))))))))

(event `InputAction|Secondary Action`
  (params (Key :type "Key Structure"))
  (bind _looking_at (`self.Looking At`))
  (bind (_returnvalue_roll _returnvalue_pitch _returnvalue_yaw) (`KismetMathLibrary.BreakRotator` (`self.K2_GetActorRotation` _looking_at)))
  (:`Pressed`
    (if (`|EnumEquality` (`self.Mode`) "NewEnumerator1")
      (`/Engine/EditorBlueprintResources/StandardMacros.IsValid` _looking_at
        (:`Is Valid`
          (`self.K2_SetActorRotation` _looking_at (`KismetMathLibrary.MakeRotator` _returnvalue_roll _returnvalue_pitch (+ _returnvalue_yaw 90.0)) false))))))

(event `Key|#`
  (params (Key :type "Key Structure"))
  (:`Pressed`
    (switch `/Game/Core/EMode` (`self.Mode`)
      (:`NewEnumerator0`
        (set `self.Mode` "NewEnumerator1"))
      (:`NewEnumerator1`
        (set `self.Mode` "NewEnumerator0")))
    (`/Game/UI/WBP_TestHUD.SetMode` (`self.HUD`) (`self.Mode`))))

(event `self.ReceiveBeginPlay`
  (bind _returnvalue (`|CreateWidget` "/Game/UI/WBP_TestHUD.WBP_TestHUD_C"))
  (`/Game/UI/WBP_TestHUD.SetMode` _returnvalue (`self.Mode`))
  (bind _output_get (set `self.HUD` _returnvalue))
  (`UserWidget.AddToViewport` _output_get 0))

(fn `Linetrace`
  (bind _lookpoint (`self.LookPoint`))
  (bind _looking_at (`self.Looking At`))
  (bind _returnvalue (`SceneComponent.K2_GetComponentLocation` _lookpoint))
  (bind (_outhit _returnvalue_2) (`KismetSystemLibrary.LineTraceSingle` :`Start` _returnvalue :`End` (+ _returnvalue (* (`KismetMathLibrary.GetForwardVector` (`SceneComponent.K2_GetComponentRotation` _lookpoint)) 100.0)) :`TraceChannel` "TraceTypeQuery1" :`DrawDebugType` "ForOneFrame"))
  (if _returnvalue_2
    (if (`KismetSystemLibrary.DoesImplementInterface` (`.HitActor` (`GameplayStatics.BreakHitResult` _outhit)) "/Game/BPI/BPI_Interact.BPI_Interact_C")
      (set `self.Look At Location` (`.TraceEnd` (`GameplayStatics.BreakHitResult` _outhit)))
      (bind _asbp_container (cast `/Game/Blueprints/BP_Container` (`.HitActor` (`GameplayStatics.BreakHitResult` _outhit)) :!pure true))
      (if (not (== (`self.Looking At`) _asbp_container))
        (`/Engine/EditorBlueprintResources/StandardMacros.IsValid` _looking_at
          (:`Is Valid`
            (`/Game/Blueprints/BP_Container.Looked At` _looking_at false))
          (:`Is Not Valid`
            _))
        (bind _output_get (set `self.Looking At` _asbp_container))
        (`/Game/Blueprints/BP_Container.Looked At` _output_get true))
      (else
        (set `self.Look At Location` (`.ImpactPoint` (`GameplayStatics.BreakHitResult` _outhit)))
        (`/Engine/EditorBlueprintResources/StandardMacros.IsValid` (`self.Looking At`) :!label _label
          (:`Is Valid`
            (`/Game/Blueprints/BP_Container.Looked At` (`self.Looking At`) false))
          (:`Is Not Valid`
            _))
        (set `self.Looking At` null)))
    (else
      (set `self.Look At Location` (`.TraceEnd` (`GameplayStatics.BreakHitResult` _outhit)))
      (goto _label))))

(fn `Snap Check`
  (locals (GridSize :type "Float (double-precision)" :default 100.0))
  (bind (_newvar_0_location _newvar_0_rotation _newvar_0_scale) (`KismetMathLibrary.BreakTransform` (`self.NewVar_0`)))
  (bind _returnvalue (`self.Round To Grid` (`self.Look At Location`)))
  (if (`self.Has Container`)
    (set `self.NewVar_0` (`KismetMathLibrary.MakeTransform` _returnvalue _newvar_0_rotation _newvar_0_scale))
    (`self.K2_SetActorLocation` (`self.Container Held`) _returnvalue false false)
    (return)))

(fn `UserConstructionScript`)