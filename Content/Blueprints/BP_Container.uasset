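; BP_Container is a base container actor that holds a single item.
; Deposit stores an item only when empty and Withdraw returns and clears it only when full, both reporting success and printing a debug message.
; Each successful transfer calls the empty ItemGiven or ItemTaken function, apparently hooks for child Blueprints.
; The Lookedat event swaps the mesh material between highlighted and wood as look focus changes.
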(event `/Game/BPI/BPI_Interact.Looked At`
  (params (`Looking At?` :type Boolean))
  (bind _staticmeshcomponent (`self.StaticMeshComponent`))
  (if `Looking At?`
    (`PrimitiveComponent.SetMaterial` _staticmeshcomponent 0 "/Game/Materials/M_Highlighted.M_Highlighted")
    (else
      (`PrimitiveComponent.SetMaterial` _staticmeshcomponent 0 "/Game/Materials/M_Wood.M_Wood"))))

(fn `Deposit`
  (params (Item :type "/Game/Core/FItem Structure"))
  (returns (Success :type Boolean))
  (`KismetSystemLibrary.PrintString` "Deposited")
  (if (`self.HasItem`)
    (return false)
    (else
      (set `self.Contents` Item)
      (`self.Item Given`)
      (set `self.HasItem` true)
      (return true))))

(fn `Item Given`)

(fn `Item Taken`)

(fn `UserConstructionScript`)

(fn `Withdraw`
  (returns (Item :type "/Game/Core/FItem Structure") (Success :type Boolean))
  (locals (`Local Content` :type "/Game/Core/FItem Structure"))
  (`KismetSystemLibrary.PrintString` "Withdrawn")
  (if (`self.HasItem`)
    (set `local.Local Content` (`self.Contents`))
    (set `self.Contents` (struct))
    (`self.Item Taken`)
    (set `self.HasItem` false)
    (return (`local.Local Content`) true)
    (else
      (return (struct) false))))